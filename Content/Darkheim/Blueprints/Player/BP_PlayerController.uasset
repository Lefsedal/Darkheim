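; Player controller for Darkheim that handles the player death sequence and toggles the player's input.
; On death it unpossesses, fades the camera to black, shows the death widget, then after a short delay removes it and restarts the level via console command.
; Custom enable and disable input events set movement, rotation and combat lock flags on the BP_Player reference cached at BeginPlay.
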(event Custom|OnDeath
  (Pawn|UnPossess)
  (CameraFades|StartCameraFade :self (Variables|Default|GetPlayerCameraManager) :ToAlpha 1.0 :Duration 1.0 :bHoldWhenFinished true)
  (bind _returnvalue (UserInterface|CreateWidget "/Game/Darkheim/Blueprints/Widgets/WG_PlayerDeath.WG_PlayerDeath_C" self))
  (UserInterface|Viewport|AddtoViewport _returnvalue 0)
  (Utilities|FlowControl|Delay 2.0)
  (Widget|RemovefromParent _returnvalue)
  (Development|ExecuteConsoleCommand "RestartLevel" 0))

(event Custom|DisableInputCustom
  (bind _as_bp_player (Variables|Default|GetAs%20BP%20Player))
  (Variables|/Game/Darkheim/Blueprints/Player/BP_Player.BP_Player_C|SetDisableMovement _as_bp_player true)
  (Variables|/Game/Darkheim/Blueprints/Player/BP_Player.BP_Player_C|SetDisableRotation _as_bp_player true)
  (Variables|/Game/Darkheim/Blueprints/Player/BP_Player.BP_Player_C|SetDisableCombat _as_bp_player true))

(event Custom|EnableInputCustom
  (bind _as_bp_player (Variables|Default|GetAs%20BP%20Player))
  (Variables|/Game/Darkheim/Blueprints/Player/BP_Player.BP_Player_C|SetDisableMovement _as_bp_player false)
  (Variables|/Game/Darkheim/Blueprints/Player/BP_Player.BP_Player_C|SetDisableRotation _as_bp_player false)
  (Variables|/Game/Darkheim/Blueprints/Player/BP_Player.BP_Player_C|SetDisableCombat _as_bp_player false))

(event EventBeginPlay
  (bind _asbp_player (Utilities|Casting|CastToBP_Player (Game|GetPlayerCharacter 0)))
  (Variables|Default|SetAs%20BP%20Player _asbp_player))

(fn ConstructionScript)