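; Enemy_AI is the AI controller for Darkheim enemies, linking the controlled BP_EnemyAI pawn to the BT_Enemy behavior tree.
; On BeginPlay it caches the pawn, runs the tree, targets the first player character and writes the current state to the AIState blackboard key.
; AIAttack switches that state and updates the blackboard, while PawnAttack forwards the attack call to the pawn.
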(event Custom|PawnAttack
  ;[1 1 1] Plays attack animation
  (Default|Attack (Variables|Default|GetAs%20BP%20Enemy%20AI)))

(event Custom|AIAttack
  (bind _output_get (Variables|Default|SetCurrentState "NewEnumerator1"))
  (AI|Components|Blackboard|SetValueasEnum (AI|GetBlackboard 0) (Utilities|Name|MakeLiteralName "AIState") _output_get))

(event EventBeginPlay
  (bind _asbp_enemy_ai (Utilities|Casting|CastToBP_EnemyAI (Pawn|GetControlledPawn)))
  (Variables|Default|SetAs%20BP%20Enemy%20AI _asbp_enemy_ai)
  (AI|RunBehaviorTree "/Game/Darkheim/Blueprints/Enemy/BT_Enemy.BT_Enemy")
  (Variables|Default|SetCurrentTarget (Game|GetPlayerCharacter 0))
  (AI|Components|Blackboard|SetValueasEnum (AI|GetBlackboard 0) (Utilities|Name|MakeLiteralName "AIState") (Variables|Default|GetCurrentState)))

(fn ConstructionScript)