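; FightDirector is a combat director that picks which enemy in EnemyList attacks, on a looping timer.
; Each enemy starts with a random grade, which every tick of that timer multiplies by a facing factor favoring forward vectors opposed to the player's.
; The top-graded enemy's Enemy_AI controller runs AIAttack, then that enemy's grade is re-randomized.
; Per-enemy debug widgets display the grades.
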(event Custom|TriggerAttack
  ;[1 1 1] Gets the enemy with the highest grade and calls AIAttack
  (CallFunction|RecalculateScores)
  (bind _loc_highestgradedai1 (CallFunction|FindHighestGrade))
  (Development|PrintString (Utilities|GetDisplayName _loc_highestgradedai1) true true "(R=1.000000,G=0.864047,B=0.000000,A=1.000000)")
  (bind _asenemy_ai (Utilities|Casting|CastToEnemy_AI (AI|GetAIController _loc_highestgradedai1)))
  (Default|AIAttack _asenemy_ai)
  (Utilities|Map|Add (Variables|Default|GetEnemyGrading) _loc_highestgradedai1 (Math|Random|RandomFloatinRange 1.0 5.0))
  (CallFunction|UpdateDebugWidgets _loc_highestgradedai1))

(event EventBeginPlay
  (for _array_element (Variables|Default|GetEnemyList)
    (CallFunction|AddDebugWidgets _array_element))
  (Utilities|Time|SetTimerbyEvent (delegate Custom|TriggerAttack) 4.0 true))

(fn ConstructionScript)

(fn FindHighestGrade
  ;[1 1 1] Loops through the EnemyGrading array and saves the highest value in a local variable
  (bind _keys (Utilities|Map|Keys (Variables|Default|GetEnemyGrading)))
  (for _array_element _keys
    (if (> (.Value (Utilities|Map|Find (Variables|Default|GetEnemyGrading) _array_element)) (LocalVariables|GetLoc_HighestValue))
      (LocalVariables|SetLoc_HighestValue (.Value (Utilities|Map|Find (Variables|Default|GetEnemyGrading) _array_element)))
      (LocalVariables|SetLoc_HighestGradedAI _array_element)))
  ;[1 1 1] Returns values to be used in the function
  (return (LocalVariables|GetLoc_HighestValue) (LocalVariables|GetLoc_HighestGradedAI)))

(fn AddDebugWidgets
  (params (EnemyInstance :type BP%20Enemy%20AI%20Object%20Reference%20%28by%20ref%29))
  ;[1 1 1] Adds the debug widget to each of the enemies
  (Utilities|Map|Add (Variables|Default|GetEnemyGrading) EnemyInstance (Math|Random|RandomFloatinRange 1.0 5.0))
  (bind _returnvalue (UserInterface|CreateWidget "/Game/Darkheim/Blueprints/Enemy/WG_DebugEnemyAI.WG_DebugEnemyAI_C" 0 EnemyInstance (.Value (Utilities|Map|Find (Variables|Default|GetEnemyGrading) EnemyInstance))))
  (Utilities|Map|Add (Variables|Default|GetEnemyWidgets) EnemyInstance _returnvalue)
  (bind _returnvalue_2 (AddComponent|AddWidgetComponent EnemyInstance false))
  (UserInterface|SetWidget _returnvalue_2 _returnvalue))

(fn UpdateDebugWidgets
  (params (EnemyInstance :type BP%20Enemy%20AI%20Object%20Reference))
  ;[1 1 1] Finds widget attached to each enemy
  (Variables|/Game/Darkheim/Blueprints/Enemy/WG_DebugEnemyAI.WG_DebugEnemyAI_C|SetFightingGrade (.Value (Utilities|Map|Find (Variables|Default|GetEnemyWidgets) EnemyInstance)) (.Value (Utilities|Map|Find (Variables|Default|GetEnemyGrading) EnemyInstance))))

(fn RecalculateScores
  (CallFunction|ScorebyPosition))

(fn ScorebyPosition
  (bind _enemygrading (Variables|Default|GetEnemyGrading))
  (for _array_element (Variables|Default|GetEnemyList)
    (Utilities|Map|Add _enemygrading _array_element (* (.Value (Utilities|Map|Find _enemygrading _array_element)) (+ (Math|Float|NormalizetoRange (* (Math|Vector|DotProduct (Transformation|GetActorForwardVector _array_element) (Transformation|GetActorForwardVector (Game|GetPlayerCharacter 0))) -1.0) -1.0 1.0) 0.5)))
    (CallFunction|UpdateDebugWidgets _array_element)))