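; Bonfire-style checkpoint actor where the player rests and saves progress.
; Overlapping its sphere caches the player, shows an interact prompt and opens a Gate for InteractwithObject; leaving removes the prompt and closes it.
; Interacting hides the prompt, records this checkpoint in the "save1" slot, rests the player, unequips weapon and shield, then saves through GM_Darkheim.
; Interacting again re-shows the prompt, toggled by NotVisible.
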(event OnComponentBeginOverlap(Sphere)
  (params (OverlappedComponent :type Primitive%20Component%20Object%20Reference) (OtherActor :type Actor%20Object%20Reference) (OtherComp :type Primitive%20Component%20Object%20Reference) (OtherBodyIndex :type Integer) (bFromSweep :type Boolean) (SweepResult :type Hit%20Result%20Structure%20%28by%20ref%29))
  (bind _asbp_player (Utilities|Casting|CastToBP_Player OtherActor))
  (Variables|Default|SetAs%20BP%20Player _asbp_player)
  (Variables|Default|SetNotVisible true)
  (bind _returnvalue (UserInterface|CreateWidget "/Game/Darkheim/Blueprints/Widgets/WG_InteractPrompt.WG_InteractPrompt_C"))
  (UserInterface|Viewport|AddtoViewport _returnvalue 0)
  (Utilities|FlowControl|Gate true) ; enters at Open
)

(event OnComponentEndOverlap(Sphere)
  (params (OverlappedComponent :type Primitive%20Component%20Object%20Reference) (OtherActor :type Actor%20Object%20Reference) (OtherComp :type Primitive%20Component%20Object%20Reference) (OtherBodyIndex :type Integer))
  (bind _as_bp_player (Variables|Default|GetAs%20BP%20Player))
  (Variables|Default|SetNotVisible false)
  (Utilities|IsValid (stale OnComponentBeginOverlap(Sphere) _returnvalue)
    (:Is%20Valid
      (Widget|RemovefromParent (stale OnComponentBeginOverlap(Sphere) _returnvalue))
      (Utilities|FlowControl|Gate true) ; enters at Close
    )))

(event EventInteractwithObject
  (bind _as_bp_player (Variables|Default|GetAs%20BP%20Player))
  (if (Variables|Default|GetNotVisible)
    (Utilities|FlowControl|Gate true
      (:Exit
        (Variables|Default|SetNotVisible false)
        (Widget|SetVisibility (stale OnComponentBeginOverlap(Sphere) _returnvalue) "Hidden")
        (Utilities|FlowControl|Sequence
          (:then_0
            ;[1 1 1] Save current checkpoint
            (bind _returnvalue (SaveGame|LoadGamefromSlot "save1"))
            (bind _asbp_save_game (Utilities|Casting|CastToBP_SaveGame _returnvalue))
            (if (not (== (Variables|/Game/Darkheim/Blueprints/BP_SaveGame.BP_SaveGame_C|GetCheckpointUsed _asbp_save_game) self))
              (Variables|/Game/Darkheim/Blueprints/BP_SaveGame.BP_SaveGame_C|SetCheckpointUsed _asbp_save_game self)
              (SaveGame|SaveGametoSlot _asbp_save_game "save1")))
          (:then_1
            ;[1 1 1] Rests at bonfire
            (Default|BonfireRest _as_bp_player)
            (Default|UnequipWeapon _as_bp_player)
            (Default|UnequipShield _as_bp_player)
            (bind _asgm_darkheim (Utilities|Casting|CastToGM_Darkheim (Game|GetGameMode)))
            (Default|SaveGame _asgm_darkheim)))))
    (else
      (Widget|SetVisibility (stale OnComponentBeginOverlap(Sphere) _returnvalue) "Visible")
      (Variables|Default|SetNotVisible true))))

(event EventBeginPlay
  (bind _as_bp_player (Variables|Default|GetAs%20BP%20Player))
  (if (Variables|Default|GetNotVisible)
    (Variables|Default|SetNotVisible true)
    (bind _returnvalue (UserInterface|CreateWidget "/Game/Darkheim/Blueprints/Widgets/WG_InteractPrompt.WG_InteractPrompt_C"))
    (UserInterface|Viewport|AddtoViewport _returnvalue 0)
    (Utilities|FlowControl|Gate true) ; enters at Open
  ))

(fn ConstructionScript)