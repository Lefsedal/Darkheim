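; Enemy AI character Blueprint for a sword-wielding foe that attacks, takes damage and dies.
; BeginPlay caches its AI controller and the player, initializes the health widget and attaches a spawned sword to the weapon socket.
; Attack plays a montage; damage lowers health, triggering either a hit reaction or death.
; The unfinished death handler stops AI logic, clears focus, disables capsule collision, resets player lock-on and destroys the lock-on sphere.
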(event Custom|Attack
  ;[1 1 1] Attack
  (Animation|Montage|PlayMontage (Variables|Character|GetMesh) "/Game/Darkheim/Assets/Animations/AllAnim/Sword_Attack_01_Montage.Sword_Attack_01_Montage"
    (:then
      (Development|PrintString (Utilities|String|Append (Utilities|GetDisplayName self) " Is Attacking") true true "(R=1.000000,G=0.000000,B=0.665606,A=1.000000)"))))

(event Custom|OnDeath
  (bind _as_enemy_ai (Variables|Default|GetAs%20Enemy%20AI))
  ;[1 1 1] On Death (Not Finished)
  (Development|PrintString (Utilities|String|Append (Utilities|GetDisplayName self) ": " "Is dead"))
  (AI|Logic|StopLogic (Variables|/Script/AIModule.AIController|GetBrainComponent _as_enemy_ai) "")
  (AI|ClearFocus _as_enemy_ai)
  (Collision|SetCollisionEnabled (Variables|Collision|GetCapsuleComponent) "NoCollision")
  (Default|ResetLockon (Variables|Default|GetAs%20BP%20Player))
  (Components|DestroyComponent (Variables|Default|GetLockOnSphere)))

(event EventBeginPlay
  ;[0.1529 0.005182 0.004777] Begin Play
  (Utilities|FlowControl|Sequence
    (:then_0
      ;[1 1 1] Saves reference to AI controller
      (bind _asenemy_ai (Utilities|Casting|CastToEnemy_AI (Pawn|GetController)))
      (Variables|Default|SetAs%20Enemy%20AI _asenemy_ai)
      ;[1 1 1] Gets reference to the player
      (bind _asbp_player (Utilities|Casting|CastToBP_Player (Game|GetPlayerCharacter 0)))
      (Variables|Default|SetAs%20BP%20Player _asbp_player))
    (:then_1
      ;[1 1 1] Update health widget
      (bind _aswg_enemy_hp (Utilities|Casting|CastToWG_EnemyHP (UserInterface|GetUserWidgetObject (Variables|Default|GetHealthWidget))))
      (Default|Init _aswg_enemy_hp self))
    (:then_2
      ;[1 1 1] Equip weapon
      (bind _returnvalue (Game|SpawnActorfromClass "/Game/Darkheim/Blueprints/BP_Paladin_Sword_Child.BP_Paladin_Sword_Child_C" (Transformation|GetSocketTransform (Variables|Character|GetMesh) "Weapon_Socket" "RTS_World") "Undefined" 0 0))
      (bind _output_get (Variables|Default|SetEquipped%20Weapon _returnvalue))
      (Transformation|AttachComponentToComponent _output_get (Variables|Character|GetMesh) "Weapon_Socket" "SnapToTarget" "SnapToTarget" "SnapToTarget" true))))

(event Game|Damage|EventAnyDamage
  (params (Damage :type Float%20%28single-precision%29) (DamageType :type Damage%20Type%20Object%20Reference) (InstigatedBy :type Controller%20Object%20Reference) (DamageCauser :type Actor%20Object%20Reference))
  ;[1 0.02417 0] Take Damage
  (bind _output_get (Variables|Default|SetHealth (- (Variables|Default|GetHealth) Damage)))
  (Development|PrintString (Utilities|String|Append (Utilities|GetDisplayName self) (Utilities|String|ToString(Float) _output_get)) true true "(R=1.000000,G=0.299270,B=0.000000,A=1.000000)")
  (if (<= (Variables|Default|GetHealth) 0.0)
    (CallFunction|OnDeath)
    (else
      (Animation|Montage|PlayMontage (Variables|Character|GetMesh) "/Game/Darkheim/Assets/Animations/AllAnim/Hit_reaction_Montage.Hit_reaction_Montage"))))

(fn ConstructionScript)