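; Frost Walker enemy character that spawns with a socketed sword and shield and fights under an AI controller.
; Attack alternates two sword montages, buffering repeat requests so AttackCombo can chain the next swing or reset.
; Damage lowers health and plays a hit reaction until death, marked unfinished, stops AI logic, disables capsule collision and notifies the player.
; It also initializes a hidden health widget and can show a lock-on circle.
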(event Custom|OnDeath
  (bind _as_enemy_ai (Variables|Default|GetAs%20Enemy%20AI))
  ;[1 1 1] On Death (Not Finished)
  (Development|PrintString (Utilities|String|Append (Utilities|GetDisplayName self) ": " "Is dead"))
  (Variables|Default|SetAI_Dead true)
  (AI|Logic|StopLogic (Variables|/Script/AIModule.AIController|GetBrainComponent _as_enemy_ai) "")
  (AI|ClearFocus _as_enemy_ai)
  (Collision|SetCollisionEnabled (Variables|Collision|GetCapsuleComponent) "NoCollision")
  (Default|SwitchonDeath (Variables|Default|GetAs%20BP%20Player))
  (Components|DestroyComponent (Variables|Default|GetHealthWidget)))

(event Custom|AttackCombo
  ;[1 1 1] Attack + Combo
  (if (Variables|Default|GetSaveAttack)
    (Variables|Default|SetSaveAttack false)
    (if (== (Variables|Default|GetAttackCount) 2)
      (Utilities|FlowControl|Delay 0.7)
      (Variables|Default|SetAttackCount 0 :!label _label)
      (Variables|Default|SetIsAttacking false)
      (else
        (switch int (Variables|Default|GetAttackCount)
          (:0
            (Variables|Default|SetAttackCount 1)
            (Animation|PlayAnimMontage "/Game/Darkheim/Assets/Animations/FrostWalker/FW_Sword_Attack_01_Montage1.FW_Sword_Attack_01_Montage1" 1.0 "None"))
          (:1
            (Variables|Default|SetAttackCount 0)
            (Animation|PlayAnimMontage "/Game/Darkheim/Assets/Animations/FrostWalker/FW_Sword_Attack_02_Montage.FW_Sword_Attack_02_Montage" 1.0 "None")))))
    (else
      (goto _label))))

(event Custom|Attack
  ;[1 1 1] Attack + Combo
  (if (Variables|Default|GetIsAttacking)
    (Variables|Default|SetSaveAttack true)
    (else
      (Variables|Default|SetIsAttacking true)
      (switch int (Variables|Default|GetAttackCount)
        (:0
          (Variables|Default|SetAttackCount 1)
          (Animation|PlayAnimMontage "/Game/Darkheim/Assets/Animations/FrostWalker/FW_Sword_Attack_01_Montage1.FW_Sword_Attack_01_Montage1" 1.0 "None"))
        (:1
          (Variables|Default|SetAttackCount 0)
          (Animation|PlayAnimMontage "/Game/Darkheim/Assets/Animations/FrostWalker/FW_Sword_Attack_02_Montage.FW_Sword_Attack_02_Montage" 1.0 "None"))))))

(event Custom|ShowLockOnCircle
  (bind _aswg_lock_on_circle (Utilities|Casting|CastToWG_LockOnCircle (UserInterface|GetUserWidgetObject (Variables|Default|GetLockOnCircle))))
  (Default|EnableCircle _aswg_lock_on_circle self))

(event EventBeginPlay
  ;[0.1529 0.005182 0.004777] Begin Play
  (Utilities|FlowControl|Sequence
    (:then_0
      ;[1 1 1] Saves reference to AI controller
      (bind _asenemy_ai (Utilities|Casting|CastToEnemy_AI (Pawn|GetController)))
      (Variables|Default|SetAs%20Enemy%20AI _asenemy_ai)
      ;[1 1 1] Gets reference to the player
      (bind _asbp_player (Utilities|Casting|CastToBP_Player (Game|GetPlayerCharacter 0)))
      (Variables|Default|SetAs%20BP%20Player _asbp_player))
    (:then_1
      ;[1 1 1] Update health widget
      (Variables|Default|SetCurrentHealth (Variables|Default|GetMaxHealth))
      (bind _aswg_enemy_hp (Utilities|Casting|CastToWG_EnemyHP (UserInterface|GetUserWidgetObject (Variables|Default|GetHealthWidget))))
      (Default|Init _aswg_enemy_hp self))
    (:then_2
      ;[1 1 1] Equip weapon
      (bind _returnvalue (Game|SpawnActorfromClass "/Game/Darkheim/Blueprints/Enemy_FrostWalker/BP_Enemy_Sword.BP_Enemy_Sword_C" (Transformation|GetSocketTransform (Variables|Character|GetMesh) "Weapon_Socket" "RTS_World") "Undefined" 0 0))
      (bind _output_get (Variables|Default|SetEquipped%20Weapon _returnvalue))
      (Transformation|AttachComponentToComponent _output_get (Variables|Character|GetMesh) "Weapon_Socket" "SnapToTarget" "SnapToTarget" "SnapToTarget" true))
    (:then_3
      ;[1 1 1] Equip weapon
      (bind _returnvalue_2 (Game|SpawnActorfromClass "/Game/Darkheim/Blueprints/Enemy_FrostWalker/BP_Enemy_Shield.BP_Enemy_Shield_C" (Transformation|GetSocketTransform (Variables|Character|GetMesh) "Shield_Socket" "RTS_World") "Undefined" 0 0))
      (bind _output_get_2 (Variables|Default|SetEquippedShield _returnvalue_2))
      (Transformation|AttachComponentToComponent _output_get_2 (Variables|Character|GetMesh) "Shield_Socket" "SnapToTarget" "SnapToTarget" "SnapToTarget" true))
    (:then_4
      (Rendering|SetVisibility (Variables|Default|GetHealthWidget) false false))))

(event Game|Damage|EventAnyDamage
  (params (Damage :type Float%20%28single-precision%29) (DamageType :type Damage%20Type%20Object%20Reference) (InstigatedBy :type Controller%20Object%20Reference) (DamageCauser :type Actor%20Object%20Reference))
  ;[1 0.02417 0] Take Damage
  (bind _output_get (Variables|Default|SetCurrentHealth (- (Variables|Default|GetCurrentHealth) Damage)))
  (Development|PrintString (Utilities|String|Append (Utilities|GetDisplayName self) (Utilities|String|ToString(Float) _output_get)) true true "(R=1.000000,G=0.299270,B=0.000000,A=1.000000)")
  (if (<= (Variables|Default|GetCurrentHealth) 0.0)
    (CallFunction|OnDeath)
    (else
      (Animation|Montage|PlayMontage (Variables|Character|GetMesh) "/Game/Darkheim/Assets/Animations/FrostWalker/FW_Hit_reaction_Montage1.FW_Hit_reaction_Montage1"))))

(fn ConstructionScript)