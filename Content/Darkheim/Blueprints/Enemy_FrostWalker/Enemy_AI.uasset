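; AI controller for the Frost Walker enemy that runs its behavior tree and bridges perception and pawn actions.
; On BeginPlay it starts BT_Enemy, caches the controlled pawn and copies its patrol path's looping flag to the blackboard.
; AI Perception updates write whether the player is sensed to CanSeePlayer.
; Custom events set the AIState blackboard enum for attacking and trigger the pawn's attack.
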(event OnTargetPerceptionUpdated(AIPerception)
  (params (Actor :type Actor%20Object%20Reference) (Stimulus :type AI%20Stimulus%20Structure))
  ;[1 1 1] Can see player
  (Utilities|Casting|CastToBP_Player Actor)
  (AI|Components|Blackboard|SetValueasBool (AI|GetBlackboard 0) (Utilities|Name|MakeLiteralName "CanSeePlayer") (.bSuccessfullySensed (Utilities|Struct|BreakAIStimulus Stimulus))))

(event Custom|PawnAttack
  ;[1 1 1] Plays attack animation
  (Default|Attack (Variables|Default|GetAs%20BP%20Enemy%20AI)))

(event Custom|AIAttack
  (bind _output_get (Variables|Default|SetCurrentState "NewEnumerator1"))
  (AI|Components|Blackboard|SetValueasEnum (AI|GetBlackboard 0) (Utilities|Name|MakeLiteralName "AIState") _output_get))

(event EventBeginPlay
  (AI|RunBehaviorTree "/Game/Darkheim/Blueprints/Enemy_FrostWalker/BT_Enemy.BT_Enemy")
  ;[1 1 1] Gets IsLooping from PatrolPath actor and sets it as PathLooping in the blackboard
  (bind _asbp_frost_walker (Utilities|Casting|CastToBP_FrostWalker (Pawn|GetControlledPawn)))
  (bind _output_get (Variables|Default|SetAs%20BP%20Enemy%20AI _asbp_frost_walker))
  (AI|Components|Blackboard|SetValueasBool (AI|GetBlackboard 0) (Utilities|Name|MakeLiteralName "PathLooping") (Variables|/Game/Darkheim/Blueprints/PatrolPath.PatrolPath_C|GetIsLooping (Variables|/Game/Darkheim/Blueprints/Enemy_FrostWalker/BP_FrostWalker.BP_FrostWalker_C|GetPatrolPath _output_get))))

(fn ConstructionScript)