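; BP_Paladin_Sword is a melee sword that deals fixed damage to actors its capsule begins overlapping, ignoring BP_Player.
; AttackStart and AttackEnd toggle an AttackReady flag that gates damage, and a DoOnce with a short delayed reset limits repeat hits.
; BeginPlay casts the player character to both BP_Player and BP_EnemyAI to store references, neither of which the damage logic uses.
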(event OnComponentBeginOverlap(Capsule)
  (params (OverlappedComponent :type Primitive%20Component%20Object%20Reference) (OtherActor :type Actor%20Object%20Reference) (OtherComp :type Primitive%20Component%20Object%20Reference) (OtherBodyIndex :type Integer) (bFromSweep :type Boolean) (SweepResult :type Hit%20Result%20Structure%20%28by%20ref%29))
  ;[1 1 1] Deal Damage
  (Utilities|Casting|CastToBP_Player OtherActor
    (:CastFailed
      (if (Variables|Default|GetAttackReady)
        (Utilities|FlowControl|DoOnce false :!label _label
          (:Completed
            (Game|Damage|ApplyDamage OtherActor 5e+01 0 0)
            (Utilities|FlowControl|Delay 0.3)
            (goto _label Reset)))))))

(event EventBeginPlay
  (bind _returnvalue (Game|GetPlayerCharacter 0))
  (bind _asbp_player (Utilities|Casting|CastToBP_Player _returnvalue))
  (Variables|Default|SetAs%20BP%20Player _asbp_player)
  (bind _asbp_enemy_ai (Utilities|Casting|CastToBP_EnemyAI _returnvalue))
  (Variables|Default|SetAs%20BP%20Enemy%20AI _asbp_enemy_ai))

(event EventAttackStart
  (Variables|Default|SetAttackReady true))

(event EventAttackEnd
  (Variables|Default|SetAttackReady false))

(fn ConstructionScript)