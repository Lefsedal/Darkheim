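; Frost King boss enemy that spawns a great axe on its weapon socket and adds a boss health widget on BeginPlay.
; Attack and AttackCombo chain two montages through a saved-attack flag and counter, resetting after the combo.
; Damage reduces health and plays a montage, or triggers an unfinished death that stops AI logic, disables capsule collision and clears the player's lock-on.
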(event Custom|Attack
  ;[1 1 1] Attack + Combo
  (if (Variables|Default|GetIsAttacking)
    (Variables|Default|SetSaveAttack true)
    (else
      (Variables|Default|SetIsAttacking true)
      (switch int (Variables|Default|GetAttackCount)
        (:0
          (Variables|Default|SetAttackCount 1)
          (Animation|PlayAnimMontage "/Game/Darkheim/Assets/Animations/FrostKing/Combat/great_sword_slash_Montage.great_sword_slash_Montage" 1.0 "None"))
        (:1
          (Variables|Default|SetAttackCount 2)
          (Animation|PlayAnimMontage "/Game/Darkheim/Assets/Animations/FrostKing/Combat/great_sword_slash__3__Montage.great_sword_slash__3__Montage" 1.0 "None"))))))

(event Custom|OnDeath
  (bind _as_ai_frost_king (Variables|Default|GetAs%20AI%20Frost%20King))
  ;[1 1 1] On Death (Not Finished)
  (Development|PrintString (Utilities|String|Append (Utilities|GetDisplayName self) ": " "Is dead"))
  (Variables|Default|SetAI_Dead true)
  (AI|Logic|StopLogic (Variables|/Script/AIModule.AIController|GetBrainComponent _as_ai_frost_king) "")
  (AI|ClearFocus _as_ai_frost_king)
  (Collision|SetCollisionEnabled (Variables|Collision|GetCapsuleComponent) "NoCollision")
  (Default|ResetLockon (Variables|Default|GetAs%20BP%20Player))
  (Components|DestroyComponent (Variables|Default|GetLockOnSphere)))

(event Custom|AttackCombo
  ;[1 1 1] Attack + Combo
  (if (Variables|Default|GetSaveAttack)
    (Variables|Default|SetSaveAttack false)
    (if (== (Variables|Default|GetAttackCount) 2)
      (Utilities|FlowControl|Delay 0.7)
      (Variables|Default|SetAttackCount 0 :!label _label)
      (Variables|Default|SetIsAttacking false)
      (else
        (switch int (Variables|Default|GetAttackCount)
          (:0
            (Variables|Default|SetAttackCount 1)
            (Animation|PlayAnimMontage "/Game/Darkheim/Assets/Animations/FrostKing/Combat/great_sword_slash_Montage.great_sword_slash_Montage" 1.0 "None"))
          (:1
            (Variables|Default|SetAttackCount 2)
            (Animation|PlayAnimMontage "/Game/Darkheim/Assets/Animations/FrostKing/Combat/great_sword_slash__3__Montage.great_sword_slash__3__Montage" 1.0 "None")))))
    (else
      (goto _label))))

(event EventBeginPlay
  ;[0.1529 0.005182 0.004777] Begin Play
  (Utilities|FlowControl|Sequence
    (:then_0
      ;[1 1 1] Saves reference to AI controller
      (bind _asai_frost_king (Utilities|Casting|CastToAI_FrostKing (Pawn|GetController)))
      (Variables|Default|SetAs%20AI%20Frost%20King _asai_frost_king)
      ;[1 1 1] Gets reference to the player
      (bind _asbp_player (Utilities|Casting|CastToBP_Player (Game|GetPlayerCharacter 0)))
      (Variables|Default|SetAs%20BP%20Player _asbp_player))
    (:then_1
      ;[1 1 1] Create health widget
      (bind _returnvalue (UserInterface|CreateWidget "/Game/Darkheim/Blueprints/Widgets/WG_BossHealth.WG_BossHealth_C"))
      (UserInterface|Viewport|AddtoViewport _returnvalue 0))
    (:then_2
      ;[1 1 1] Sets variables
      (Variables|Default|SetCurrentHealth (Variables|Default|GetMaxHealth)))
    (:then_3
      ;[1 1 1] Equip weapon
      (bind _returnvalue_2 (Game|SpawnActorfromClass "/Game/Darkheim/Blueprints/Enemy_FrostKing/BP_Enemy_GreatAxe.BP_Enemy_GreatAxe_C" (Transformation|GetSocketTransform (Variables|Character|GetMesh) "Weapon_Socket" "RTS_World") "Undefined" 0 0))
      (bind _output_get (Variables|Default|SetEquippedWeapon _returnvalue_2))
      (Transformation|AttachComponentToComponent _output_get (Variables|Character|GetMesh) "Weapon_Socket" "SnapToTarget" "SnapToTarget" "SnapToTarget" true))))

(event Game|Damage|EventAnyDamage
  (params (Damage :type Float%20%28single-precision%29) (DamageType :type Damage%20Type%20Object%20Reference) (InstigatedBy :type Controller%20Object%20Reference) (DamageCauser :type Actor%20Object%20Reference))
  ;[1 0.02417 0] Take Damage
  (Variables|Default|SetCurrentHealth (- (Variables|Default|GetCurrentHealth) Damage))
  (if (<= (Variables|Default|GetCurrentHealth) 0.0)
    (CallFunction|OnDeath)
    (else
      (Animation|Montage|PlayMontage (Variables|Character|GetMesh) 0))))

(fn ConstructionScript)