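; Trigger volume that starts the Frost King boss fight when the player walks into its box.
; On first overlap it spawns BP_FrostKing with its behavior tree at a SpawnLocation actor, using a HasSpawned flag on the game instance to prevent respawns.
; After a short delay it has the game mode create the boss health bar and closes the first BP_BossDoor found in the level.
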(event OnComponentBeginOverlap(Box)
  (params (OverlappedComponent :type Primitive%20Component%20Object%20Reference) (OtherActor :type Actor%20Object%20Reference) (OtherComp :type Primitive%20Component%20Object%20Reference) (OtherBodyIndex :type Integer) (bFromSweep :type Boolean) (SweepResult :type Hit%20Result%20Structure%20%28by%20ref%29))
  (bind _spawnlocation (Variables|Default|GetSpawnLocation))
  (Utilities|Casting|CastToBP_Player OtherActor)
  (bind _asbp_instance (Utilities|Casting|CastToBP_Instance (Game|GetGameInstance)))
  (if (not (Variables|/Game/Darkheim/Blueprints/BP_Instance.BP_Instance_C|GetHasSpawned _asbp_instance))
    (AI|SpawnAIFromClass "/Game/Darkheim/Blueprints/Enemy_FrostKing/BP_FrostKing.BP_FrostKing_C" "/Game/Darkheim/Blueprints/Enemy_FrostKing/BT_FrostKing.BT_FrostKing" (Transformation|GetActorLocation _spawnlocation) (Transformation|GetActorRotation _spawnlocation) false 0)
    (Variables|/Game/Darkheim/Blueprints/BP_Instance.BP_Instance_C|SetHasSpawned _asbp_instance true)
    (Utilities|FlowControl|Delay 0.2)
    (bind _asgm_darkheim (Utilities|Casting|CastToGM_Darkheim (Game|GetGameMode)))
    (Default|CreateBossHealthBar _asgm_darkheim)
    (bind _outactors (Actor|GetAllActorsOfClass "/Game/Darkheim/Blueprints/Enemy_FrostKing/BP_BossDoor.BP_BossDoor_C"))
    (Default|CloseDoor (Utilities|Array|Get(acopy) _outactors))))

(fn ConstructionScript)