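; Behavior tree task that gives a BP_FrostWalker its next patrol destination.
; On execute it sets walk speed to patrol pace, reads the patrol path point at the blackboard index, and writes its world-space location to the blackboard vector.
; It finishes successfully only with a valid path; a failed cast or missing path never calls FinishExecute.
; An AI focus-clearing branch is left disconnected.
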(event EventReceiveExecuteAI
  (params (OwnerController :type AI%20Controller%20Object%20Reference) (ControlledPawn :type Pawn%20Object%20Reference))
  (bind _asbp_frost_walker (Utilities|Casting|CastToBP_FrostWalker ControlledPawn))
  (Variables|/Script/Engine.CharacterMovementComponent|SetMaxWalkSpeed (Variables|/Script/Engine.Character|GetCharacterMovement _asbp_frost_walker) 2e+02)
  (bind _patrolpath (Variables|/Game/Darkheim/Blueprints/Enemy_FrostWalker/BP_FrostWalker.BP_FrostWalker_C|GetPatrolPath _asbp_frost_walker)
    (:then
      (AI|BehaviorTree|SetBlackboardValueasVector (Variables|Default|GetBB_PathVector) (Math|Transform|TransformLocation (Transformation|GetActorTransform _patrolpath) (Utilities|Array|Get(acopy) (Variables|/Game/Darkheim/Blueprints/PatrolPath.PatrolPath_C|GetPathPoints _patrolpath) (Class|BTFunctionLibrary|GetBlackboardValueasInt (Variables|Default|GetBB_PathIndex)))))
      (AI|BehaviorTree|FinishExecute true))
    (:else)))