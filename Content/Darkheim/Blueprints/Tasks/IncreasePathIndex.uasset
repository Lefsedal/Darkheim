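; Behavior tree task that advances a Frost Walker's patrol path index on the blackboard.
; It casts the controlled pawn to BP_FrostWalker and compares the next index with the last index of its PatrolPath points.
; If in range it writes the incremented index and succeeds; otherwise it fails without resetting, and a failed cast never finishes the task.
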(event EventReceiveExecuteAI
  (params (OwnerController :type AI%20Controller%20Object%20Reference) (ControlledPawn :type Pawn%20Object%20Reference))
  (bind _bb_pathindex (Variables|Default|GetBB_PathIndex))
  (bind _returnvalue (Class|BTFunctionLibrary|GetBlackboardValueasInt _bb_pathindex))
  (bind _returnvalue_2 (+ _returnvalue 1))
  (bind _asbp_frost_walker (Utilities|Casting|CastToBP_FrostWalker ControlledPawn))
  (if (<= _returnvalue_2 (Utilities|Array|LastIndex (Variables|/Game/Darkheim/Blueprints/PatrolPath.PatrolPath_C|GetPathPoints (Variables|/Game/Darkheim/Blueprints/Enemy_FrostWalker/BP_FrostWalker.BP_FrostWalker_C|GetPatrolPath _asbp_frost_walker))))
    (Class|BTFunctionLibrary|SetBlackboardValueasInt (Variables|Default|GetBB_PathIndex) _returnvalue_2)
    (AI|BehaviorTree|FinishExecute true)
    (else
      (AI|BehaviorTree|FinishExecute false))))