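; Behavior tree task that picks a navigable move target around the player for an AI pawn and stores it in the blackboard.
; It offsets from near the player by Distance along a random direction within the hemisphere facing the pawn, then samples a nearby navigable point.
; It also applies WalkSpeed, focuses the player only if a camera-channel trace hits them, otherwise clears focus, then finishes successfully.
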(event EventReceiveExecuteAI
  (params (OwnerController :type AI%20Controller%20Object%20Reference) (ControlledPawn :type Pawn%20Object%20Reference))
  (Variables|Default|SetController OwnerController)
  (Variables|Default|SetPawn ControlledPawn)
  (AI|BehaviorTree|SetBlackboardValueasVector (Variables|Default|GetBB_TargetLocation) (.RandomLocation (Class|NavigationSystemV1|GetRandomPointinNavigableRadius (+ (- (Transformation|GetActorLocation (Game|GetPlayerCharacter 0)) "30.000000, 0,30.000000") (* (Math|Random|RandomUnitVectorinConeinDegrees (Math|Vector|GetUnitDirection(Vector) (Transformation|GetActorLocation (Game|GetPlayerCharacter 0)) (Transformation|GetActorLocation ControlledPawn)) 9e+01) (Variables|Default|GetDistance))) 1e+02 0 0)))
  (CallFunction|SetWalkSpeed)
  (CallFunction|SetFocus)
  (AI|BehaviorTree|FinishExecute true))

(fn SetWalkSpeed
  (bind _ascharacter (Utilities|Casting|CastToCharacter (Variables|Default|GetPawn)))
  (Variables|/Script/Engine.CharacterMovementComponent|SetMaxWalkSpeed (Variables|/Script/Engine.Character|GetCharacterMovement _ascharacter) (Variables|Default|GetWalkSpeed)))

(fn SetFocus
  (bind _pawn (Variables|Default|GetPawn))
  (bind _controller (Variables|Default|GetController))
  (bind _outhit (Collision|LineTraceByChannel (Transformation|GetActorLocation _pawn) (Transformation|GetActorLocation (Game|GetPlayerCharacter 0)) "TraceTypeQuery2" false (Utilities|Array|MakeArray _pawn) "None"))
  (if (== (.hitactor _outhit) (Game|GetPlayerCharacter 0))
    (AI|SetFocus _controller (.hitactor _outhit))
    (else
      (AI|ClearFocus _controller))))