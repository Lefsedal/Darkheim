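; Darkheim game mode that handles checkpoint-based saving, loading and respawning through a single save slot.
; BeginPlay creates the save if missing or moves the player beside the saved checkpoint, caches player, FrostWalker and checkpoint references, then respawns if the saved-location flag is set.
; Respawn destroys the player, spawns and possesses a new one at that checkpoint.
; Other events toggle the flag, restart the level, delete the save or reset input.
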(event Custom|InputReset
  (bind _returnvalue (Game|GetPlayerController 0))
  ;[1 1 1] Call to reset input (OLD, Need revisit)
  (Input|EnableInput (Variables|Default|GetAs%20BP%20Player) _returnvalue)
  (Input|SetInputModeGameandUI _returnvalue 0 "DoNotLock" false)
  (Variables|/Script/Engine.PlayerController|SetbShowMouseCursor _returnvalue false))

(event Custom|Save%20Game
  ;[1 1 1] Save Game
  (bind _returnvalue (SaveGame|LoadGamefromSlot "save1"))
  (bind _asbp_save_game (Utilities|Casting|CastToBP_SaveGame _returnvalue))
  (Variables|/Game/Darkheim/Blueprints/BP_SaveGame.BP_SaveGame_C|SetUseSavedLocation _asbp_save_game true)
  (SaveGame|SaveGametoSlot _asbp_save_game "save1"))

(event Custom|Respawn
  ;[1 1 1] Respawn player at last interacted checkpoint
  (bind _returnvalue (SaveGame|LoadGamefromSlot "save1"))
  (bind _asbp_save_game (Utilities|Casting|CastToBP_SaveGame _returnvalue))
  (Actor|DestroyActor (Variables|Default|GetAs%20BP%20Player))
  (bind _returnvalue_2 (Game|SpawnActorfromClass "/Game/Darkheim/Blueprints/Player/BP_Player.BP_Player_C" (Transformation|GetActorTransform (Variables|/Game/Darkheim/Blueprints/BP_SaveGame.BP_SaveGame_C|GetCheckpointUsed _asbp_save_game)) "AlwaysSpawn" 0 0))
  (Pawn|Possess (Game|GetPlayerController 0) _returnvalue_2))

(event Custom|Load%20Game
  ;[1 1 1] Load Game
  (Development|ExecuteConsoleCommand "RestartLevel" 0))

(event Custom|ChangeLevels
  ;[1 1 1] Change level
  (bind _returnvalue (SaveGame|LoadGamefromSlot "save1"))
  (bind _asbp_save_game (Utilities|Casting|CastToBP_SaveGame _returnvalue))
  (Variables|/Game/Darkheim/Blueprints/BP_SaveGame.BP_SaveGame_C|SetUseSavedLocation _asbp_save_game false)
  (SaveGame|SaveGametoSlot _asbp_save_game "save1"))

(event Custom|DeleteSaveGame
  ;[1 1 1] Delete Save game
  (SaveGame|DeleteGameinSlot "save1"))

(event EventBeginPlay
  ;[0.9842 0 1] Begin Play
  (Utilities|FlowControl|Sequence
    (:then_0
      (bind _returnvalue (SaveGame|DoesSaveGameExist "save1"))
      (if _returnvalue
        (bind _returnvalue_2 (SaveGame|LoadGamefromSlot "save1"))
        (bind _asbp_save_game (Utilities|Casting|CastToBP_SaveGame _returnvalue_2))
        (Utilities|IsValid (Variables|/Game/Darkheim/Blueprints/BP_SaveGame.BP_SaveGame_C|GetCheckpointUsed _asbp_save_game) ; NotValid = Spawns player at player start
          (:Is%20Valid
            ;[1 1 1] Load game functionality
            ;;[1 1 1] Move player to last used checkpoint
            (bind _asbp_player (Utilities|Casting|CastToBP_Player (Game|GetPlayerCharacter 0)))
            (Transformation|SetWorldTransform (Variables|/Script/Engine.Actor|GetRootComponent _asbp_player) (Math|Transform|MakeTransform (- (.Location (Math|Transform|BreakTransform (Transformation|GetActorTransform (Variables|/Game/Darkheim/Blueprints/BP_SaveGame.BP_SaveGame_C|GetCheckpointUsed _asbp_save_game)))) "100.000000, 0,0.000000") (.Rotation (Math|Transform|BreakTransform (Transformation|GetActorTransform (Variables|/Game/Darkheim/Blueprints/BP_SaveGame.BP_SaveGame_C|GetCheckpointUsed _asbp_save_game)))) (.Scale (Math|Transform|BreakTransform (Transformation|GetActorTransform (Variables|/Game/Darkheim/Blueprints/BP_SaveGame.BP_SaveGame_C|GetCheckpointUsed _asbp_save_game))))) false false)))
        (else
          ;[1 1 1] Create save file
          (bind _returnvalue_3 (SaveGame|CreateSaveGameObject "/Game/Darkheim/Blueprints/BP_SaveGame.BP_SaveGame_C"))
          (SaveGame|SaveGametoSlot _returnvalue_3 "save1"))))
    (:then_1
      ;[1 1 1] Object reference
      (Utilities|FlowControl|Sequence
        (:then_0
          (bind _outactors (Actor|GetAllActorsOfClass "/Game/Darkheim/Blueprints/Enemy_FrostWalker/BP_FrostWalker.BP_FrostWalker_C"))
          (Variables|Default|SetAs%20FrostWalker _outactors)
          (bind _outactors_2 (Actor|GetAllActorsOfClass "/Game/Darkheim/Blueprints/BP_Checkpoint.BP_Checkpoint_C"))
          (Variables|Default|SetCheckpoints _outactors_2))
        (:then_1
          (bind _asbp_player_2 (Utilities|Casting|CastToBP_Player (Game|GetPlayerCharacter 0)))
          (Variables|Default|SetAs%20BP%20Player _asbp_player_2))
        (:then_2
          (bind _returnvalue_4 (SaveGame|LoadGamefromSlot "save1"))
          (bind _asbp_save_game_2 (Utilities|Casting|CastToBP_SaveGame _returnvalue_4))
          (if (Variables|/Game/Darkheim/Blueprints/BP_SaveGame.BP_SaveGame_C|GetUseSavedLocation _asbp_save_game_2)
            (CallFunction|Respawn)))))))

(fn ConstructionScript)